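; Sliding door variant of a key-locked door parent, layering movement, sound and lock-colour feedback onto the inherited open, close and key logic.
; Open and Close play or reverse one timeline, rate-scaled by TimeToOpen, that slides the door and rotates its lock.
; Construction creates dynamic materials for lock and frame and tints frame lights.
; Key overrides refresh lock colour; RemoveKey always passes 1 to the parent, ignoring Amount.
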(event Custom|SlideClosed
  (Audio|PlaySoundatLocation (Variables|SlidingDoor|GetCloseDoorSound) (Transformation|GetActorLocation) "0, 0, 0" 1.0 1.0 0.0 0 0 0 0)
  (CallFunction|SetLockColour (CallFunction|IsUnlocked))
  (bind (_direction _alpha _lockopenalpha) (Timeline|TL_RiseLower Reverse)
    (:Update
      (Transformation|SetRelativeLocation (Variables|Default|GetTransform) (Math|Vector|Lerp(Vector) "0, 0, 0" (Variables|SlidingDoor|GetSlideOpenLocation) _alpha) false false)
      (Transformation|SetRelativeRotation (Variables|Default|GetLockTransform) (Math|Rotator|Lerp(Rotator) "0, 0, 0" "0.000000,0.000000,180.000000" _lockopenalpha) false false))))

(event Custom|SlideOpen
  (Audio|PlaySoundatLocation (Variables|SlidingDoor|GetOpenDoorSound) (Transformation|GetActorLocation) "0, 0, 0" 1.0 1.0 0.0 0 0 0 0)
  (CallFunction|SetLockColour true)
  (bind (_direction _alpha _lockopenalpha) (Timeline|TL_RiseLower Play)
    (:Update
      (Transformation|SetRelativeLocation (Variables|Default|GetTransform) (Math|Vector|Lerp(Vector) "0, 0, 0" (Variables|SlidingDoor|GetSlideOpenLocation) _alpha) false false)
      (Transformation|SetRelativeRotation (Variables|Default|GetLockTransform) (Math|Rotator|Lerp(Rotator) "0, 0, 0" "0.000000,0.000000,180.000000" _lockopenalpha) false false))))

(event EventBeginPlay
  (|CallParentFunction)
  (Components|Timeline|SetPlayRate (Variables|Default|GetTL_RiseLower) (/ 1.0 (Variables|SlidingDoor|GetTimeToOpen))))

(fn ConstructionScript
  (|CallParentFunction)
  (CallFunction|SetDoorMatInstance)
  (CallFunction|SetDoorFrameMatInstance)
  (CallFunction|SetLockColour (CallFunction|IsUnlocked))
  (Rendering|Components|Light|SetLightColor (Variables|Default|GetFrameLight2) (Variables|SlidingDoor|GetDoorLightColour) true)
  (Rendering|Material|SetVectorParameterValue (Variables|Default|GetDoorFrameMatInstance) "Emissive2Tint" (Variables|SlidingDoor|GetDoorLightColour) :!class /Script/Engine.MaterialInstanceDynamic))

(fn Open
  (|CallParentFunction)
  (CallFunction|SlideOpen))

(fn Close
  (|CallParentFunction)
  (CallFunction|SlideClosed))

(fn SetDoorMatInstance
  (bind _lockmesh (Variables|Default|GetLockMesh))
  (bind _returnvalue (Rendering|Material|GetMaterial _lockmesh 0))
  (if (and (Utilities|IsValid _lockmesh) (Utilities|IsValid _returnvalue))
    (bind _returnvalue_2 (Rendering|Material|CreateDynamicMaterialInstance _lockmesh 0 _returnvalue "None" :!class /Script/Engine.PrimitiveComponent))
    (Variables|Default|SetLockMatInstance _returnvalue_2)))

(fn SetLockColour
  (params (bUnlocked :type Boolean))
  (bind _lockmatinstance (Variables|Default|GetLockMatInstance)
    (:then
      (Rendering|Material|SetVectorParameterValue _lockmatinstance "EmissiveTint" (Math|Color|SelectColor (Variables|SlidingDoor|GetUnlockedColour) (Variables|SlidingDoor|GetLockedColour) bUnlocked) :!class /Script/Engine.MaterialInstanceDynamic))
    (:else)))

(fn AddKey
  (|CallParentFunction)
  (CallFunction|SetLockColour (CallFunction|IsUnlocked)))

(fn AddKeys
  (params (KeysCollected :type Integer))
  (|CallParentFunction KeysCollected)
  (CallFunction|SetLockColour (CallFunction|IsUnlocked)))

(fn OnSpecialKeyCollected
  (|CallParentFunction)
  (CallFunction|SetLockColour true))

(fn SetDoorFrameMatInstance
  (bind _doorframe (Variables|Default|GetDoorFrame))
  (bind _returnvalue (Rendering|Material|GetMaterial _doorframe 0))
  (if (and (Utilities|IsValid _doorframe) (Utilities|IsValid _returnvalue))
    (bind _returnvalue_2 (Rendering|Material|CreateDynamicMaterialInstance _doorframe 0 _returnvalue "None" :!class /Script/Engine.PrimitiveComponent))
    (Variables|Default|SetDoorFrameMatInstance _returnvalue_2)))

(fn RemoveKey
  (params (Amount :type Integer))
  (|CallParentFunction 1)
  (CallFunction|SetLockColour (CallFunction|IsUnlocked)))

(fn OnKeysCollected
  (|CallParentFunction)
  (CallFunction|SetLockColour (CallFunction|IsUnlocked)))